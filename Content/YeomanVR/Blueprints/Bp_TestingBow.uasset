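; Prototype two-handed VR bow: the first controller to grip holds it at that hand's grip socket, and a second becomes the draw hand.
; While drawn, Tick aims the bow along the line between controllers and bends both string halves back by their scale-adjusted distance.
; Releasing the draw hand snaps the string to its construction-computed nock midpoint and resets rotation once.
; Dropping the bow detaches it, with physics left off as a workaround.
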(event `self.ReceiveTick`
  (params (DeltaSeconds :type "Float (single-precision)"))
  (bind _returnvalue_x (`KismetMathLibrary.BreakVector` (`self.GetActorScale3D`)))
  (bind (_stringmidpoint_x _stringmidpoint_y _stringmidpoint_z) (`KismetMathLibrary.BreakVector` (`self.StringMidpoint`)))
  (bind _bowhand (`self.BowHand`))
  (bind (_returnvalue_roll _returnvalue_pitch _returnvalue_yaw) (`KismetMathLibrary.BreakRotator` (`SceneComponent.K2_GetComponentRotation` _bowhand)))
  ;[1 1 1] Bow Prototype Partially Based on following Tutorial
  ;;[1 1 1] Should keep bow align with the two controllers
  (bind _drawhand (`self.DrawHand`)
    (:`then`
      (bind (_returnvalue_roll_2 _returnvalue_pitch_2) (`KismetMathLibrary.BreakRotator` (`KismetMathLibrary.FindLookAtRotation` (`SceneComponent.K2_GetComponentLocation` _drawhand) (`SceneComponent.K2_GetComponentLocation` _bowhand))))
      (`self.K2_SetActorRelativeRotation` (`KismetMathLibrary.MakeRotator` _returnvalue_roll_2 _returnvalue_pitch_2 _returnvalue_yaw))
      (`SplineMeshComponent.SetEndPosition` (`self.UpperString`) (`KismetMathLibrary.MakeVector` (/ (`KismetMathLibrary.Vector_Distance` (`SceneComponent.K2_GetComponentLocation` (`self.BowHand`)) (`SceneComponent.K2_GetComponentLocation` (`self.DrawHand`))) _returnvalue_x) _stringmidpoint_y _stringmidpoint_z) true)
      (`SplineMeshComponent.SetEndPosition` (`self.LowerString`) (`KismetMathLibrary.MakeVector` (/ (`KismetMathLibrary.Vector_Distance` (`SceneComponent.K2_GetComponentLocation` (`self.BowHand`)) (`SceneComponent.K2_GetComponentLocation` (`self.DrawHand`))) _returnvalue_x) _stringmidpoint_y _stringmidpoint_z) true)
      (goto _label :!via `Reset`))
    (:`else`
      ;;[1 1 1] Snap back string and reset rotation
      (`/Engine/EditorBlueprintResources/StandardMacros.DoOnce` true :!label _label
        (:`Completed`
          (`SplineMeshComponent.SetEndPosition` (`self.LowerString`) (`self.StringMidpoint`) true)
          (`SplineMeshComponent.SetEndPosition` (`self.UpperString`) (`self.StringMidpoint`) true)
          (`self.K2_SetActorRelativeRotation` (struct)))))))

(event `/Game/Interface/BPI_Grip.Grip`
  (params (MotionController :type "MotionControllerComponent Object Reference"))
  ;[1 1 1] Bow Prototype Partially Based on following Tutorial
  (bind _output_get (set `self.bSimPhysics` (`SceneComponent.IsSimulatingPhysics` (`self.RiserMesh`) "None")))
  (if _output_get
    (`PrimitiveComponent.SetSimulatePhysics` (`self.RiserMesh`) false))
  ;;[1 1 1] If there is no MC for the bow grip, set it
  (bind _bowhand (`self.BowHand`)
    (:`then`
      ;;[1 1 1] If there is then set the grapping hand as the one drawing the bow
      (if (!= _bowhand MotionController)
        (set `self.DrawHand` MotionController)))
    (:`else`
      (set `self.BowHand` MotionController)
      (bind _asbp_vrcharacter (cast `/Game/YeomanVR/Blueprints/BP_VRCharacter` (`GameplayStatics.GetPlayerCharacter` 0)))
      (if (== MotionController (`/Game/YeomanVR/Blueprints/BP_VRCharacter.LeftMotionController` _asbp_vrcharacter))
        (`self.K2_AttachToComponent` (`/Game/YeomanVR/Blueprints/BP_VRCharacter.LeftHand` _asbp_vrcharacter) "Bow_Grip_Socket" "SnapToTarget" "SnapToTarget" "KeepWorld")
        (else
          (`self.K2_AttachToComponent` (`/Game/YeomanVR/Blueprints/BP_VRCharacter.RightHand` _asbp_vrcharacter) "Bow_Grip_Socket" "SnapToTarget" "SnapToTarget" "KeepWorld"))))))

(event `/Game/Interface/BPI_Grip.Drop`
  (params (MotionController :type "MotionControllerComponent Object Reference"))
  ;[1 1 1] Bow Prototype Partially Based on following Tutorial
  (if (== MotionController (`self.DrawHand`))
    ;;[1 1 1] If draw hand release set to null, if bow hand release set both to null and drop object
    (set `self.DrawHand` null)
    (else
      (set `self.BowHand` null)
      (set `self.DrawHand` null)
      (`self.K2_DetachFromActor` "KeepWorld" "KeepWorld" "KeepWorld")
      ;;[1 1 1] Temp disabled until I can figure out a way for the string to not freak out
      (if (not (`self.bSimPhysics`))
        (`PrimitiveComponent.SetSimulatePhysics` (`self.RiserMesh`) false)))))

(fn `UserConstructionScript`
  (bind _relativelocation (`SceneComponent.RelativeLocation` (`self.UpperNock`)))
  (bind _relativelocation_2 (`SceneComponent.RelativeLocation` (`self.LowerNock`)))
  (bind _output_get (set `self.StringMidpoint` (+ _relativelocation (* (/ (`KismetMathLibrary.Vector_Distance` _relativelocation _relativelocation_2) 2.0) (`KismetMathLibrary.GetForwardVector` (`KismetMathLibrary.FindLookAtRotation` _relativelocation _relativelocation_2))))))
  (`SplineMeshComponent.SetStartAndEnd` (`self.UpperString`) _relativelocation (0.0 0.0 0.0) _output_get (0.0 0.0 0.0) true)
  (`SplineMeshComponent.SetStartAndEnd` (`self.LowerString`) _relativelocation_2 (0.0 0.0 0.0) _output_get (0.0 0.0 0.0) true))