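; Bp_VRSlider is a VR slider that a motion controller grips and drags along a track.
; Grip stores the controller, and Drop is set up to clear that reference on release.
; While a controller is held, Tick snaps SliderMesh to the closest point to it on the straight segment between SliderSpline's first two points, ignoring any curvature.
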(event `/Game/Interface/BPI_Grip.Grip`
  (params (MotionController :type "MotionControllerComponent Object Reference"))
  (set `self.Motion Controller` MotionController))

(event `/Game/Interface/BPI_Grip.Drop`
  (params (MotionController :type "MotionControllerComponent Object Reference"))
  (if (== (`self.Motion Controller`) MotionController)
    (set `self.Motion Controller` null)))

(event `self.ReceiveTick`
  (params (DeltaSeconds :type "Float (single-precision)"))
  (bind _sliderspline (`self.SliderSpline`))
  (bind _motion_controller (`self.Motion Controller`)
    (:`then`
      (`SceneComponent.K2_SetWorldLocation` (`self.SliderMesh`) (`KismetMathLibrary.FindClosestPointOnSegment` (`SceneComponent.K2_GetComponentLocation` _motion_controller) (`SplineComponent.GetLocationAtSplinePoint` _sliderspline 0 "World") (`SplineComponent.GetLocationAtSplinePoint` _sliderspline 1 "World")) false false))
    (:`else`)))

(fn `UserConstructionScript`)