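; VR compound bow actor that the player grips, draws and fires with motion controllers.
; The first Grip snaps the bow to that hand's socket; a later Grip near the string spawns and attaches an arrow.
; Tick gets draw length from C++ using the draw hand's position.
; Alternate releases the arrow with force from a draw curve and plays right-hand haptics, while Drop from the bow hand detaches it.
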(event `self.ReceiveTick`
  (params (DeltaSeconds :type "Float (single-precision)"))
  ;[1 1 1] Use c++ to get the draw length.
  (bind _drawhand (`self.DrawHand`)
    (:`then`
      (bind _output_get (set `self.DrawLength` (`self.GetDrawLength` (`SceneComponent.K2_GetComponentLocation` _drawhand))))
      (`KismetSystemLibrary.PrintText` (`KismetTextLibrary.Conv_DoubleToText` _output_get "HalfToEven")))
    (:`else`)))

(event `/Game/YeomanVR/InterfaceEnums/BPI_Grip.Grip`
  (params (MotionController :type "MotionControllerComponent Object Reference"))
  (bind _bowskeleton (`self.BowSkeleton`))
  (`self.BowHand` ; If !Valid then grip bow, if it is valid grab string
    (:`then`
      (bind _returnvalue (`self.ShouldSpawnArrow` (`SceneComponent.K2_GetComponentLocation` MotionController)))
      (`KismetSystemLibrary.PrintString` (`KismetStringLibrary.Conv_BoolToString` _returnvalue))
      (if _returnvalue
        (set `self.DrawHand` MotionController)
        (`self.SpawnArrow`)
        (`self.AttachArrow`)))
    (:`else`
      ;[1 1 1] Attach bow grip to hand that sent Grip Message
      (bind _asbp_vrcharacter (cast `/Game/YeomanVR/Blueprints/BP_VRCharacter` (`GameplayStatics.GetPlayerCharacter` 0)))
      (set `self.BowHand` MotionController)
      (bind _output_get (set `self.As BP VRCharacter` _asbp_vrcharacter))
      (if (== (`self.BowHand`) (`/Game/YeomanVR/Blueprints/BP_VRCharacter.LeftMotionController` _asbp_vrcharacter))
        (`self.K2_AttachToComponent` (`/Game/YeomanVR/Blueprints/BP_VRCharacter.LeftHand` _output_get) "Bow_Grip_Socket" "SnapToTarget" "SnapToTarget" "KeepWorld")
        (`SceneComponent.K2_AddLocalRotation` _bowskeleton (struct :`Yaw` 90.0) false false)
        (else
          (`self.K2_AttachToComponent` (`/Game/YeomanVR/Blueprints/BP_VRCharacter.RightHand` _output_get) "Bow_Grip_Socket" "SnapToTarget" "SnapToTarget" "KeepWorld")))
      (`PrimitiveComponent.SetSimulatePhysics` _bowskeleton false))))

(event `/Game/YeomanVR/InterfaceEnums/BPI_Grip.Alternate`
  (bind _as_bp_vrcharacter (`self.As BP VRCharacter`))
  (bind _returnvalue (`self.GetDrawValue` (`CurveFloat.GetFloatValue` (`self.draw force curve`) (`self.DrawLength`))))
  ;[1 1 1] Release Arrow
  (set `self.DrawHand` null)
  (if (== (`/Game/YeomanVR/Blueprints/BP_VRCharacter.LeftMotionController` _as_bp_vrcharacter) (`self.BowHand`))
    (`self.ReleaseArrow` (`/Game/YeomanVR/Blueprints/BP_VRCharacter.LeftHand` _as_bp_vrcharacter) _returnvalue)
    (else
      (`self.ReleaseArrow` (`/Game/YeomanVR/Blueprints/BP_VRCharacter.RightHand` _as_bp_vrcharacter) _returnvalue)))
  (set `self.DrawLength` 0.0)
  (`OculusXRInputFunctionLibrary.PlayCurveHapticEffect` "/Game/YeomanVR/Blueprints/Archery/HFC_Compound.HFC_Compound" "Right"))

(event `/Game/YeomanVR/InterfaceEnums/BPI_Grip.Drop`
  (params (MotionController :type "MotionControllerComponent Object Reference"))
  (if (== MotionController (`self.BowHand`))
    (set `self.DrawHand` null)
    (set `self.BowHand` null)
    (`self.K2_DetachFromActor` "KeepWorld" "KeepWorld" "KeepWorld")
    (set `self.DrawLength` 0.0)
    (`PrimitiveComponent.SetCollisionEnabled` (`self.BowSkeleton`) "QueryAndPhysics")))

(fn `UserConstructionScript`)