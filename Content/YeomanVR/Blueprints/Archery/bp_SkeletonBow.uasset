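; VR skeletal bow actor that can be gripped, drawn and fired with two motion controllers.
; The first grip snaps it to that hand's socket; a second grip near enough, per ShouldSpawnArrow, becomes the draw hand and attaches a new arrow.
; Tick derives draw length from the draw hand's offset in string-socket space.
; Alternate releases the arrow with curve-mapped draw force; Drop detaches the bow and restores physics collision.
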(event `/Game/YeomanVR/InterfaceEnums/BPI_Grip.Grip`
  (params (MotionController :type "MotionControllerComponent Object Reference"))
  ;[1 1 1] PickUp/Drop
  (`self.BowHand`
    (:`then`
      (bind _returnvalue (`self.ShouldSpawnArrow` (`SceneComponent.K2_GetComponentLocation` MotionController)))
      (if _returnvalue
        (`KismetSystemLibrary.PrintString` "Setting Draw Hand")
        (set `self.DrawHand` MotionController)
        (bind _returnvalue_2 (`self.SpawnArrow`))
        (set `self.ArrowRef` _returnvalue_2)
        (`self.AttachArrow`)))
    (:`else`
      (set `self.BowHand` MotionController)
      (bind _asbp_vrcharacter (cast `/Game/YeomanVR/Blueprints/BP_VRCharacter` (`GameplayStatics.GetPlayerCharacter` 0)))
      (if (== (`/Game/YeomanVR/Blueprints/BP_VRCharacter.LeftMotionController` _asbp_vrcharacter) MotionController)
        (`self.K2_AttachToComponent` (`/Game/YeomanVR/Blueprints/BP_VRCharacter.LeftHand` _asbp_vrcharacter) "Bow_Grip_Socket" "SnapToTarget" "SnapToTarget" "KeepWorld")
        (else
          (`self.K2_AttachToComponent` (`/Game/YeomanVR/Blueprints/BP_VRCharacter.RightHand` _asbp_vrcharacter) "Bow_Grip_Socket" "SnapToTarget" "SnapToTarget" "KeepWorld")))
      (`PrimitiveComponent.SetCollisionEnabled` (`self.BowSkeleton`) "QueryOnly"))))

(event `/Game/YeomanVR/InterfaceEnums/BPI_Grip.Drop`
  (params (MotionController :type "MotionControllerComponent Object Reference"))
  ;[1 1 1] PickUp/Drop
  (`self.K2_DetachFromActor` "KeepWorld" "KeepWorld" "KeepWorld")
  (set `self.DrawLength_0` 0.0)
  (set `self.DrawHand` null)
  (set `self.BowHand` null)
  (`PrimitiveComponent.SetCollisionEnabled` (`self.BowSkeleton`) "QueryAndPhysics"))

(event `/Game/YeomanVR/InterfaceEnums/BPI_Grip.Alternate`
  (bind _returnvalue (`KismetMathLibrary.MapRangeClamped` (`CurveFloat.GetFloatValue` (`self.DrawForceCurve`) (`self.DrawLength_0`)) 1.0 1.0 20.0 2000.0))
  ;[1 1 1 1 12] Used to calculate velocity via a draw force curve, allowing a shorter draw to produce a slower arrow. Using my 45# Longbow as an example, average arrow speed is around 87m/s. Velocity in UE is calculated in UU. 1 UU == 1 CM (1000 = 1m/s). So maximum value in the clamp should ve 8700
  (set `self.DrawHand` null)
  (bind _asbp_vrcharacter (cast `/Game/YeomanVR/Blueprints/BP_VRCharacter` (`GameplayStatics.GetPlayerCharacter` 0)))
  (if (== (`/Game/YeomanVR/Blueprints/BP_VRCharacter.LeftMotionController` _asbp_vrcharacter) (`self.BowHand`))
    (`self.ReleaseArrow` (`/Game/YeomanVR/Blueprints/BP_VRCharacter.LeftHand` _asbp_vrcharacter) _returnvalue)
    (else
      (`self.ReleaseArrow` (`/Game/YeomanVR/Blueprints/BP_VRCharacter.RightHand` _asbp_vrcharacter) _returnvalue)))
  (set `self.DrawLength_0` 0.0))

(event `self.ReceiveTick`
  (params (DeltaSeconds :type "Float (single-precision)"))
  ;[1 1 1] Get distance between Draw Hand MC and the string socket. Set this as the draw length we will use this to influence arrow velo.
  (bind _drawhand (`self.DrawHand`)
    (:`then`
      (bind _returnvalue_x (`KismetMathLibrary.BreakVector` (`KismetMathLibrary.InverseTransformLocation` (`SceneComponent.GetSocketTransform` (`self.BowSkeleton`) "StringIdle" "RTS_World") (`SceneComponent.K2_GetComponentLocation` _drawhand))))
      (set `self.DrawLength_0` (`KismetMathLibrary.MapRangeClamped` (`KismetMathLibrary.FClamp` _returnvalue_x 0.0 38.0) 38.0 0.0 1.0)))
    (:`else`)))

(fn `UserConstructionScript`)