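; Wooden arrow for VR archery that the player can grip and drop.
; Grip turns off mesh physics, stores the motion controller and snaps the arrow to the Bow_Grip_Socket on player 0's right hand, whichever controller gripped it.
; Drop detaches it at its current world transform if the controller is valid, without re-enabling physics, and otherwise prints a debug message.
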(event `/Game/Interface/BPI_Grip.Grip`
  (params (MotionController :type "MotionControllerComponent Object Reference"))
  (bind _mesh (`self.Mesh`))
  (if (`SceneComponent.IsAnySimulatingPhysics` _mesh)
    (`PrimitiveComponent.SetSimulatePhysics` _mesh false))
  (set `self.MotionController` MotionController)
  (bind _asbp_vrcharacter (cast `/Game/YeomanVR/Blueprints/BP_VRCharacter` (`GameplayStatics.GetPlayerCharacter` 0)))
  (`self.K2_AttachToComponent` (`/Game/YeomanVR/Blueprints/BP_VRCharacter.RightHand` _asbp_vrcharacter) "Bow_Grip_Socket" "SnapToTarget" "SnapToTarget" "KeepWorld"))

(event `/Game/Interface/BPI_Grip.Drop`
  (params (MotionController :type "MotionControllerComponent Object Reference"))
  (`/Engine/EditorBlueprintResources/StandardMacros.IsValid` MotionController
    (:`Is Valid`
      (`self.K2_DetachFromActor` "KeepWorld" "KeepWorld" "KeepWorld"))
    (:`Is Not Valid`
      (`KismetSystemLibrary.PrintString` "Not Valid" true true (struct :`G` 0.66 :`B` 1.0 :`A` 1.0) 10.0))))

(fn `UserConstructionScript`)