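; BP_Trad is a grippable VR bow that tracks a bow hand and a draw hand.
; The first Grip attaches it to the matching character hand's Bow_Grip_Socket; a later Grip sets DrawHand only when the controller equals BowHand.
; Drop from DrawHand calls ReleaseArrow, while any other Drop clears both hands and detaches the bow.
; String drawing is unfinished: DrawString is empty and Tick only casts the player character.
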(event `self.ReceiveTick`
  (params (DeltaSeconds :type "Float (single-precision)"))
  (`self.DrawHand`
    (:`then`
      (cast `/Game/YeomanVR/Blueprints/BP_VRCharacter` (`GameplayStatics.GetPlayerCharacter` 0)))
    (:`else`)))

(event `/Game/Interface/BPI_Grip.Grip`
  (params (MotionController :type "MotionControllerComponent Object Reference"))
  (bind _bowhand (`self.BowHand`)
    (:`then`
      (if (== MotionController _bowhand)
        (set `self.DrawHand` MotionController)
        (bind _asbp_vrcharacter (cast `/Game/YeomanVR/Blueprints/BP_VRCharacter` (`GameplayStatics.GetPlayerCharacter` 0)))))
    (:`else`
      ;[1 1 1] If Grabbing bow then decide which hand to attach to
      (set `self.BowHand` MotionController)
      (bind _asbp_vrcharacter_2 (cast `/Game/YeomanVR/Blueprints/BP_VRCharacter` (`GameplayStatics.GetPlayerCharacter` 0)))
      (if (== (`/Game/YeomanVR/Blueprints/BP_VRCharacter.LeftMotionController` _asbp_vrcharacter_2) MotionController)
        (`self.K2_AttachToComponent` (`/Game/YeomanVR/Blueprints/BP_VRCharacter.LeftHand` _asbp_vrcharacter_2) "Bow_Grip_Socket" "SnapToTarget" "SnapToTarget" "KeepWorld")
        (else
          (`self.K2_AttachToComponent` (`/Game/YeomanVR/Blueprints/BP_VRCharacter.RightHand` _asbp_vrcharacter_2) "Bow_Grip_Socket" "SnapToTarget" "SnapToTarget" "KeepWorld"))))))

(event `/Game/Interface/BPI_Grip.Drop`
  (params (MotionController :type "MotionControllerComponent Object Reference"))
  (if (== MotionController (`self.DrawHand`))
    (set `self.DrawHand` null)
    (`self.ReleaseArrow`)
    (else
      (set `self.BowHand` null)
      (set `self.DrawHand` null)
      (`self.K2_DetachFromActor` "KeepWorld" "KeepWorld" "KeepWorld"))))

(fn `DrawString`
  (params (DrawHand :type "MotionControllerComponent Object Reference")))

(fn `UserConstructionScript`)