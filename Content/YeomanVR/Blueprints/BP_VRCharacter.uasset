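; VR player character with hand gestures, object gripping and smooth locomotion on a floor-level tracking origin.
; Grip input overlaps a sphere at each hand and sends grip/drop messages to the first BPI_Grip actor found.
; Inputs also set fist and grab animation flags; BeginPlay caches both hand AnimBPs.
; Movement follows HMD direction with deadzones; a toggle flashes text and switches off smooth yaw turning, but snap-turn logic is unwired.
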(event `InputAction|Animation_GrabLeft`
  (params (Key :type "Key Structure"))
  ;[1 1 1] Gesture Controls
  ;;[0.06918 0.9203 1] Left Fist Anim Controls
  (:`Pressed`
    (if (and (`PlayerController.IsInputKeyDown` (`GameplayStatics.GetPlayerController` 0) (stale `InputAction|Anim_TriggerLeft` Key)) (`PlayerController.IsInputKeyDown` (`GameplayStatics.GetPlayerController` 0) Key)) :!label _label
      (set `self.bLeftFistAnim` true)))
  (:`Released`
    (set `self.bLeftFistAnim` false :!label _label_2)))

(event `self.ReceiveBeginPlay`
  ;[1 1 1] Ensures HMD does not end up in floor
  (`HeadMountedDisplayFunctionLibrary.SetTrackingOrigin` "Floor")
  ;[1 1 1] Hand Animation code, based on this tutorial (https://www.youtube.com/watch?v=mee_6vlWZ8c)
  (bind _asbp_hand_animations (cast `/Game/YeomanVR/GFX/VR/Animations/BP_HandAnimations` (`SkeletalMeshComponent.GetAnimInstance` (`self.LeftHand`))))
  (set `self.leftHandAnimations` _asbp_hand_animations)
  (bind _asbp_hand_animations_2 (cast `/Game/YeomanVR/GFX/VR/Animations/BP_HandAnimations` (`SkeletalMeshComponent.GetAnimInstance` (`self.RightHand`))))
  (set `self.rightHandAnimations` _asbp_hand_animations_2))

(event `InputAction|Anim_TriggerLeft`
  (params (Key :type "Key Structure"))
  ;[1 1 1] Gesture Controls
  ;;[0.06918 0.9203 1] Left Fist Anim Controls
  (:`Pressed`
    (goto _label))
  (:`Released`
    (goto _label_2)))

(event `InputAction|LeftGrip`
  (params (Key :type "Key Structure"))
  (bind _leftsphere (`self.LeftSphere`))
  ;[1 0.08142 0] Grip Code
  (:`Pressed`
    (set `self.bLeftGrabAnim` true)
    ;;[1 1 1] Basic Grip Left
    (bind _outactors (`KismetSystemLibrary.SphereOverlapActors` (`SceneComponent.K2_GetComponentLocation` _leftsphere) (`SphereComponent.SphereRadius` _leftsphere) (`|MakeArray` "ObjectTypeQuery2" :!type "EObjectTypeQuery Enum")))
    (for _array_element _outactors
      (if (`KismetSystemLibrary.DoesImplementInterface` _array_element "/Game/Interface/BPI_Grip.BPI_Grip_C")
        (message `/Game/Interface/BPI_Grip.Grip` _array_element (`self.LeftMotionController`))
        (set `self.GrabbedActor(Left)` _array_element)
        (break))))
  (:`Released`
    (set `self.bLeftGrabAnim` false)
    (bind _grabbedactor_left_ (`self.GrabbedActor(Left)`)
      (:`then`
        (message `/Game/Interface/BPI_Grip.Drop` _grabbedactor_left_ (`self.LeftMotionController`))
        (set `self.GrabbedActor(Left)` null))
      (:`else`))))

(event `InputAction|Animation_GrabRight`
  (params (Key :type "Key Structure"))
  ;[1 1 1] Gesture Controls
  ;;[0 0.8831 1] Right Fist anim controls
  (:`Pressed`
    (if (and (`PlayerController.IsInputKeyDown` (`GameplayStatics.GetPlayerController` 0) Key) (`PlayerController.IsInputKeyDown` (`GameplayStatics.GetPlayerController` 0) (stale `InputAction|Anim_TriggerRight` Key))) :!label _label_3
      (set `self.bRightFistAnim` true)))
  (:`Released`
    (set `self.bRightFistAnim` false :!label _label_4)))

(event `InputAction|Anim_TriggerRight`
  (params (Key :type "Key Structure"))
  ;[1 1 1] Gesture Controls
  ;;[0 0.8831 1] Right Fist anim controls
  (:`Pressed`
    (goto _label_3))
  (:`Released`
    (goto _label_4)))

(event `InputAction|Right Grip`
  (params (Key :type "Key Structure"))
  (bind _rightsphere (`self.RightSphere`))
  ;[1 0.08142 0] Grip Code
  (:`Pressed`
    (set `self.bRightGrabAnim` true)
    ;;[1 1 1] Basic Grip Right
    (bind _outactors (`KismetSystemLibrary.SphereOverlapActors` (`SceneComponent.K2_GetComponentLocation` _rightsphere) (`SphereComponent.SphereRadius` _rightsphere) (`|MakeArray` "ObjectTypeQuery2" :!type "EObjectTypeQuery Enum")))
    (for _array_element _outactors
      (if (`KismetSystemLibrary.DoesImplementInterface` _array_element "/Game/Interface/BPI_Grip.BPI_Grip_C")
        (message `/Game/Interface/BPI_Grip.Grip` _array_element (`self.RightMotionController`))
        (set `self.GrabbedActor(Right)` _array_element)
        (break))))
  (:`Released`
    (set `self.bRightGrabAnim` false)
    (bind _grabbedactor_right_ (`self.GrabbedActor(Right)`)
      (:`then`
        (message `/Game/Interface/BPI_Grip.Drop` _grabbedactor_right_ (`self.RightMotionController`))
        (set `self.GrabbedActor(Right)` null))
      (:`else`))))

(event `InputAxis|Forward`
  (params (AxisValue :type "Float (single-precision)"))
  ;[1 1 1] Smooth Locomotion
  (if (> (`KismetMathLibrary.Abs` AxisValue) (`self.MovementDeadzone`))
    (`self.AddMovementInput` (`SceneComponent.GetForwardVector` (`self.HMD`)) (* AxisValue (`self.MovementSpeed`)))))

(event `InputAxis|Turn`
  (params (AxisValue :type "Float (single-precision)"))
  ;[1 1 1] Smooth Locomotion and Snap turning(disabled for now)
  (if (not (`self.bisUsingSnapTurn`))
    ;;[1 0 0] Simple smooth turn, works by rotating cam. Seems to work fine for now
    (if (> AxisValue (`self.TurningDeadzone`))
      (`self.AddControllerYawInput` (* AxisValue (`self.SmoothRotSpeed`)))
      (elif (< AxisValue (* (`self.TurningDeadzone`) -1.0))
        (`self.AddControllerYawInput` (* AxisValue (`self.SmoothRotSpeed`)))))))

(event `InputAxis|Strafe`
  (params (AxisValue :type "Float (single-precision)"))
  ;[1 1 1] Smooth Locomotion
  (if (> (`KismetMathLibrary.Abs` AxisValue) (`self.MovementDeadzone`))
    (`self.AddMovementInput` (`SceneComponent.GetRightVector` (`self.HMD`)) (* AxisValue (`self.MovementSpeed`)))))

(event `self.ReceiveTick`
  (params (DeltaSeconds :type "Float (single-precision)"))
  (set `self.DeltaTime` DeltaSeconds))

(event `InputAction|SwapLocomotion`
  (params (Key :type "Key Structure"))
  (bind _txt_locomotion (`self.TXT_Locomotion`))
  (bind _txt_locomotion_2 (`self.TXT_Locomotion`))
  ;[1 0.02348 0] Rotation Type Toggle
  (:`Pressed`
    (if (`self.bisUsingSnapTurn`)
      (set `self.bisUsingSnapTurn` false)
      (`SceneComponent.SetVisibility` _txt_locomotion true false)
      (`TextRenderComponent.K2_SetText` _txt_locomotion (`self.TXT_SnapDisbaled`))
      (`KismetSystemLibrary.Delay` 0.5)
      (`SceneComponent.SetVisibility` _txt_locomotion false false)
      (else
        (set `self.bisUsingSnapTurn` true)
        (`SceneComponent.SetVisibility` _txt_locomotion_2 true false)
        (`TextRenderComponent.K2_SetText` _txt_locomotion_2 (`self.TXT_SnapEnabled`))
        (`KismetSystemLibrary.Delay` 0.5)
        (`SceneComponent.SetVisibility` _txt_locomotion_2 false false)))))

(fn `UserConstructionScript`)