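; VR bow actor that the player grips and drops with motion controllers.
; The first Grip suspends mesh physics, records the bow hand and snaps the bow to that hand's Bow_Grip_Socket on BP_VRCharacter.
; Drop by that hand detaches it and restores prior physics.
; Draw-hand support is unfinished: a second grip only clears DrawHand, and logic attaching a hand to ArrowNockPoint is unwired.
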(event `/Game/Interface/BPI_Grip.Grip`
  (params (MotionController :type "MotionControllerComponent Object Reference"))
  (bind _bowmesh (`self.BowMesh`))
  ;[1 1 1] Grip Bow Event
  (bind _output_get (set `self.bIsSimPhysics` (`SceneComponent.IsSimulatingPhysics` _bowmesh "None")))
  (if _output_get
    (`PrimitiveComponent.SetSimulatePhysics` _bowmesh false))
  (bind _bowhand (`self.BowHand`)
    (:`then`
      ;;[1 1 1] If Already Grippped, then set as draw hand
      (if (!= _bowhand MotionController)
        (set `self.DrawHand` null)))
    (:`else`
      (set `self.BowHand` MotionController)
      ;;[1 1 1] Determine what and is gripping
      (bind _asbp_vrcharacter (cast `/Game/YeomanVR/Blueprints/BP_VRCharacter` (`GameplayStatics.GetPlayerCharacter` 0)))
      (if (== MotionController (`/Game/YeomanVR/Blueprints/BP_VRCharacter.LeftMotionController` _asbp_vrcharacter))
        (`self.K2_AttachToComponent` (`/Game/YeomanVR/Blueprints/BP_VRCharacter.LeftHand` _asbp_vrcharacter) "Bow_Grip_Socket" "SnapToTarget" "SnapToTarget" "KeepWorld")
        (else
          (`self.K2_AttachToComponent` (`/Game/YeomanVR/Blueprints/BP_VRCharacter.RightHand` _asbp_vrcharacter) "Bow_Grip_Socket" "SnapToTarget" "SnapToTarget" "KeepWorld"))))))

(event `/Game/Interface/BPI_Grip.Drop`
  (params (MotionController :type "MotionControllerComponent Object Reference"))
  (if (== MotionController (`self.DrawHand`))
    ;[1 1 1] If draw hand release set to null, if bow hand release set both to null and drop object
    (set `self.DrawHand` null)
    (else
      (set `self.BowHand` null)
      (set `self.DrawHand` null)
      (`self.K2_DetachFromActor` "KeepWorld" "KeepWorld" "KeepWorld")
      (if (`self.bIsSimPhysics`)
        (`PrimitiveComponent.SetSimulatePhysics` (`self.BowMesh`) true)))))

(fn `UserConstructionScript`)