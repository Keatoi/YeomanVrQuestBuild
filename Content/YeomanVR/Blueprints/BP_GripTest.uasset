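; BP_GripTest is a test actor for gripping and dropping a physics object with a VR motion controller.
; Grip turns off physics simulation on the static mesh, stores the controller and attaches to it, keeping the world transform.
; Drop detaches the mesh and re-enables physics if the stored controller is valid, otherwise it prints a debug message.
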(event `/Game/Interface/BPI_Grip.Grip`
  (params (MotionController :type "MotionControllerComponent Object Reference"))
  (if (`SceneComponent.IsAnySimulatingPhysics` (`self.StaticMesh`))
    (`PrimitiveComponent.SetSimulatePhysics` (`self.StaticMesh`) false))
  (set `self.Motion Controller` MotionController)
  (`self.K2_AttachToComponent` MotionController "None" "KeepWorld" "KeepWorld" "KeepWorld"))

(event `/Game/Interface/BPI_Grip.Drop`
  (params (MotionController :type "MotionControllerComponent Object Reference"))
  (`/Engine/EditorBlueprintResources/StandardMacros.IsValid` (`self.Motion Controller`)
    (:`Is Valid`
      (`SceneComponent.K2_DetachFromComponent` (`self.StaticMesh`) "KeepWorld" "KeepWorld" "KeepWorld" true)
      (`PrimitiveComponent.SetSimulatePhysics` (`self.StaticMesh`) true))
    (:`Is Not Valid`
      (`KismetSystemLibrary.PrintString` "Not Valid"))))

(fn `UserConstructionScript`)